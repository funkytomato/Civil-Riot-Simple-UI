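; Base NPC character built from placeholder shapes, with a temperament that reacts to crowding by other NPCs.
; A looping timer raises temperament while INT_NPC actors occupy the comfort zone, otherwise lowers it; capsule hits also raise it.
; Temperament tints Civilians via a dynamic material and timeline, and near maximum sends a Retreat event to the AI StateTree.
; Timelines rescale the mesh for stand/sit/lie postures; class events swap shape and colour, though their test timers are disconnected.
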(event OnComponentHit(CapsuleComponent)
  (params (HitComponent :type Primitive%20Component%20Object%20Reference) (OtherActor :type Actor%20Object%20Reference) (OtherComp :type Primitive%20Component%20Object%20Reference) (NormalImpulse :type Vector :default "0, 0, 0") (Hit :type Hit%20Result%20Structure%20%28by%20ref%29))
  ;[0.005594 0.1356 0.15 0.5] Comfort zone
  (if (not (== OtherActor self))
    (if (Utilities|DoesObjectImplementInterface OtherActor "/Game/MyContent/AI/Interfaces/INT_NPC.INT_NPC_C")
      (CallFunction|IncreaseTemperament)
      (Default|CallTemperamentUpdated))))

(event OnComponentBeginOverlap(ComfortZone)
  (params (OverlappedComponent :type Primitive%20Component%20Object%20Reference) (OtherActor :type Actor%20Object%20Reference) (OtherComp :type Primitive%20Component%20Object%20Reference) (OtherBodyIndex :type Integer) (bFromSweep :type Boolean) (SweepResult :type Hit%20Result%20Structure%20%28by%20ref%29))
  ;[0.005594 0.1356 0.15 0.5] Comfort zone
  (if (not (== OtherActor self))
    (if (Utilities|DoesObjectImplementInterface OtherActor "/Game/MyContent/AI/Interfaces/INT_NPC.INT_NPC_C")
      (Utilities|Array|AddUnique (Variables|ComfortZone|GetActorsWithinComfortZone) 0))))

(event OnComponentEndOverlap(ComfortZone)
  (params (OverlappedComponent :type Primitive%20Component%20Object%20Reference) (OtherActor :type Actor%20Object%20Reference) (OtherComp :type Primitive%20Component%20Object%20Reference) (OtherBodyIndex :type Integer))
  (bind _actorswithincomfortzone (Variables|ComfortZone|GetActorsWithinComfortZone))
  ;[0.005594 0.1356 0.15 0.5] Comfort zone
  (if (not (== OtherActor self))
    (if (Utilities|DoesObjectImplementInterface OtherActor "/Game/MyContent/AI/Interfaces/INT_NPC.INT_NPC_C")
      (Utilities|Array|RemoveIndex _actorswithincomfortzone (Utilities|Array|FindItem _actorswithincomfortzone OtherActor))
      (if (<= (Utilities|Array|Length _actorswithincomfortzone) 1)
        (Utilities|Array|Clear (Variables|ComfortZone|GetActorsWithinComfortZone))))))

(event Custom|ChangeToStandPosture
  (bind _impactpoint (CallFunction|GetGroundLocation))
  (bind _impactpoint_2 (CallFunction|GetGroundLocation))
  (bind (_x _y _z) (Math|Vector|BreakVector _impactpoint))
  (bind (_x_2 _y_2 _z_2) (Math|Vector|BreakVector _impactpoint_2))
  ;[0.1278 0.02547 0.15 0.5] Posture
  ;;[0.15 0.15 0.15 0.5] Stand Up
  (Development|PrintString "To Stand")
  (bind _scale (Timeline|TimelineForStand PlayFromStart)
    (:Update
      (Transformation|SetWorldScale3D (Variables|Default|GetCharacterPose) (Math|Vector|MakeVector 0.5 0.5 (Math|Float|Lerp (Utilities|Select :Index (Variables|Posture|GetCurrentPosture) :NewEnumerator0 (Variables|Posture|GetPoseStandHeight) :NewEnumerator1 (Variables|Posture|GetPoseSitHeight) :NewEnumerator2 (Variables|Posture|GetPoseLyedown)) (Variables|Posture|GetPoseStandHeight) _scale)))
      (Transformation|SetWorldLocation (Variables|Default|GetCharacterPose) (Math|Vector|MakeVector _x _y (+ (+ _z (Variables|Posture|GetStandOffset)) (Math|Float|Lerp (Utilities|Select :Index (Variables|Posture|GetCurrentPosture) :NewEnumerator0 (Variables|Posture|GetPoseStandHeight) :NewEnumerator1 (Variables|Posture|GetPoseSitHeight) :NewEnumerator2 (Variables|Posture|GetPoseLyedown)) (Variables|Posture|GetPoseStandHeight) _scale))) false false))
    (:Finished
      (Transformation|SetWorldLocation (Variables|Default|GetCharacterPose) (Math|Vector|MakeVector _x_2 _y_2 (Variables|Posture|GetStandOffset)) false false)
      (Variables|Posture|SetCurrentPosture "NewEnumerator0")
      (Default|CallStandFinished))))

(event Custom|ChangeToSitPosture
  (bind _impactpoint (CallFunction|GetGroundLocation))
  (bind _impactpoint_2 (CallFunction|GetGroundLocation))
  (bind (_x _y _z) (Math|Vector|BreakVector _impactpoint))
  (bind (_x_2 _y_2 _z_2) (Math|Vector|BreakVector _impactpoint_2))
  ;[0.1278 0.02547 0.15 0.5] Posture
  ;;[0.15 0.15 0.15 0.5] Sit Down
  (Development|PrintString "To Sit")
  (bind _scale (Timeline|TimelineForSit PlayFromStart)
    (:Update
      (Transformation|SetWorldScale3D (Variables|Default|GetCharacterPose) (Math|Vector|MakeVector 0.5 0.5 (Math|Float|Lerp (Utilities|Select :Index (Variables|Posture|GetCurrentPosture) :NewEnumerator0 (Variables|Posture|GetPoseStandHeight) :NewEnumerator1 (Variables|Posture|GetPoseSitHeight) :NewEnumerator2 (Variables|Posture|GetPoseLyedown)) (Variables|Posture|GetPoseSitHeight) _scale)))
      (Transformation|SetWorldLocation (Variables|Default|GetCharacterPose) (Math|Vector|MakeVector _x_2 _y_2 (+ (+ _z_2 (Variables|Posture|GetSitOffset)) (Math|Float|Lerp (Utilities|Select :Index (Variables|Posture|GetCurrentPosture) :NewEnumerator0 (Variables|Posture|GetPoseStandHeight) :NewEnumerator1 (Variables|Posture|GetPoseSitHeight) :NewEnumerator2 (Variables|Posture|GetPoseLyedown)) (Variables|Posture|GetPoseSitHeight) _scale))) false false))
    (:Finished
      (Transformation|SetWorldLocation (Variables|Default|GetCharacterPose) (Math|Vector|MakeVector _x _y (+ _z (Variables|Posture|GetSitOffset))) false false)
      (Variables|Posture|SetCurrentPosture "NewEnumerator1")
      (Default|CallSitFinished))))

(event Custom|CharacterClassChange
  ;[0.1073 0.15 0.141 0.5] Initialisation
  ;;[0.15 0.15 0.15 0.5] Character Class changer for testing
  (Utilities|FlowControl|Sequence
    (:then_0
      (switch Utilities|FlowControl|Switch|SwitchonE_CharacterClass (Variables|Character|GetCharacter%20Class)
        (:NewEnumerator0
          (Variables|Character|SetCharacter%20Class "NewEnumerator1"))
        (:NewEnumerator1
          (Variables|Character|SetCharacter%20Class "NewEnumerator2"))
        (:NewEnumerator2
          (Variables|Character|SetCharacter%20Class "NewEnumerator3"))
        (:NewEnumerator3
          (Variables|Character|SetCharacter%20Class "NewEnumerator0"))))
    (:then_1
      (CallFunction|UpdateClass))))

(event Custom|AgitateTimer
  ;[0.1073 0.15 0.141 0.5] Initialisation
  ;;[0.15 0.15 0.15 0.5] Agitator for Testing purposes
  (CallFunction|TemperamentColour))

(event Custom|TemperamentColour
  ;[0.1278 0.02547 0.15 0.5] Posture
  ;;[0.15 0.15 0.15 0.5] Temperament
  (if (Utilities|Enum|Equal(Enum) (Variables|Character|GetCharacter%20Class) "NewEnumerator0")
    (bind _agitatecolour (Timeline|AgitateTimeline SetNewTime)
      (:Update
        (Rendering|Material|SetVectorParameterValue (Variables|Stats|GetNPCMaterial) "Color" _agitatecolour :!class /Script/Engine.MaterialInstanceDynamic)))))

(event Custom|UpdateClass
  ;[0.15 0.15 0.15 0.5] Character Class
  (switch Utilities|FlowControl|Switch|SwitchonE_CharacterClass (Variables|Character|GetCharacter%20Class)
    (:NewEnumerator0
      (CallFunction|ChangeClasstoCivilian))
    (:NewEnumerator1
      (CallFunction|ChangeClasstoTrader))
    (:NewEnumerator2
      (CallFunction|ChangeClasstoPreacher))
    (:NewEnumerator3
      (CallFunction|ChangeClasstoThug))))

(event Custom|ProcessComfortZone
  ;[0.005594 0.1356 0.15 0.5] Comfort zone
  ;;[0.15 0.15 0.15 0.5] Process Comfort Zone
  (if (Utilities|Array|IsNotEmpty (Variables|ComfortZone|GetActorsWithinComfortZone))
    (CallFunction|IncreaseTemperament)
    (CallFunction|TemperamentColour)
    (Default|CallTemperamentUpdated)
    (else
      (CallFunction|DecreaseTemperament)
      (CallFunction|TemperamentColour)
      (Default|CallTemperamentUpdated))))

(event Custom|ChangeToLyingdownPosture
  (bind _impactpoint (CallFunction|GetGroundLocation))
  (bind _impactpoint_2 (CallFunction|GetGroundLocation))
  (bind (_x _y _z) (Math|Vector|BreakVector _impactpoint))
  (bind (_x_2 _y_2 _z_2) (Math|Vector|BreakVector _impactpoint_2))
  ;[0.1278 0.02547 0.15 0.5] Posture
  ;;[0.15 0.15 0.15 0.5] Lie Down
  (Development|PrintString "To lye down")
  (bind _scale (Timeline|TimelineForLyingdown PlayFromStart)
    (:Update
      (Transformation|SetWorldScale3D (Variables|Default|GetCharacterPose) (Math|Vector|MakeVector 0.5 0.5 (Math|Float|Lerp (Utilities|Select :Index (Variables|Posture|GetCurrentPosture) :NewEnumerator0 (Variables|Posture|GetPoseStandHeight) :NewEnumerator1 (Variables|Posture|GetPoseSitHeight) :NewEnumerator2 (Variables|Posture|GetPoseLyedown)) (Variables|Posture|GetPoseLyedown) _scale)))
      (Transformation|SetWorldLocation (Variables|Default|GetCharacterPose) (Math|Vector|MakeVector _x _y (+ (+ _z (Variables|Posture|GetLyingOffset)) (Math|Float|Lerp (Utilities|Select :Index (Variables|Posture|GetCurrentPosture) :NewEnumerator0 (Variables|Posture|GetPoseStandHeight) :NewEnumerator1 (Variables|Posture|GetPoseSitHeight) :NewEnumerator2 (Variables|Posture|GetPoseLyedown)) (Variables|Posture|GetPoseLyedown) _scale))) false false))
    (:Finished
      (Transformation|SetWorldLocation (Variables|Default|GetCharacterPose) (Math|Vector|MakeVector _x_2 _y_2 (+ _z_2 (Variables|Posture|GetLyingOffset))) false false)
      (Variables|Posture|SetCurrentPosture "NewEnumerator2")
      (Default|CallLieDownFinished))))

(event Custom|PostureTimer
  ;[0.15 0.15 0.15 0.5] Posture Changer for Testing
  (Utilities|FlowControl|Sequence
    (:then_0
      (switch Utilities|FlowControl|Switch|Switchone_CharacterPose (Variables|Posture|GetCurrentPosture)
        (:NewEnumerator0
          (Variables|Posture|SetTargetPosture "NewEnumerator1"))
        (:NewEnumerator1
          (Variables|Posture|SetTargetPosture "NewEnumerator2"))
        (:NewEnumerator2
          (Variables|Posture|SetTargetPosture "NewEnumerator0"))))
    (:then_1
      (bind _asnpc_aic (Utilities|Casting|CastToNPC_AIC (AI|GetAIController self)))
      (Gameplay|StateTree|SendStateTreeEvent (Variables|/Game/MyContent/AI/Controllers/NPC_AIC.NPC_AIC_C|GetStateTreeAI _asnpc_aic) (Utilities|Struct|MakeStateTreeEvent "(TagName=\"Pose.PostureChange\")") :!class /Script/GameplayStateTreeModule.StateTreeComponent))))

(event Custom|InterrogateComfortZone
  ;[0.1073 0.15 0.141 0.5] Initialisation
  ;;[0.15 0.15 0.15 0.5] Create Timer for Comfort Zone detection
  (CallFunction|ProcessComfortZone))

(event Custom|ChangeClassToCivilian
  ;[0.15 0.15 0.15 0.5] Character Class
  (Components|StaticMesh|SetStaticMesh (Variables|Default|GetCharacterPose) "/Engine/BasicShapes/MyCylinder.MyCylinder")
  (Rendering|Material|SetVectorParameterValue (Variables|Stats|GetNPCMaterial) "Color" "(R=1.000000,G=1.000000,B=1.000000,A=1.000000)" :!class /Script/Engine.MaterialInstanceDynamic))

(event Custom|ChangeClassToTrader
  ;[0.15 0.15 0.15 0.5] Character Class
  (Components|StaticMesh|SetStaticMesh (Variables|Default|GetCharacterPose) "/Engine/BasicShapes/Sphere.Sphere")
  (Rendering|Material|SetVectorParameterValue (Variables|Stats|GetNPCMaterial) "Color" "(R=1.000000,G=0.720733,B=0.000353,A=1.000000)" :!class /Script/Engine.MaterialInstanceDynamic))

(event Custom|ChangeClassToPreacher
  ;[0.15 0.15 0.15 0.5] Character Class
  (Components|StaticMesh|SetStaticMesh (Variables|Default|GetCharacterPose) "/Engine/BasicShapes/Cone.Cone")
  (Rendering|Material|SetVectorParameterValue (Variables|Stats|GetNPCMaterial) "Color" "(R=0.006999,G=1.000000,B=0.939799,A=1.000000)" :!class /Script/Engine.MaterialInstanceDynamic))

(event Custom|ChangeClassToThug
  ;[0.15 0.15 0.15 0.5] Character Class
  (Components|StaticMesh|SetStaticMesh (Variables|Default|GetCharacterPose) "/Engine/BasicShapes/Cube1.Cube1")
  (Rendering|Material|SetVectorParameterValue (Variables|Stats|GetNPCMaterial) "Color" "(R=0.000000,G=0.000000,B=0.000000,A=1.000000)" :!class /Script/Engine.MaterialInstanceDynamic))

(event EventBeginPlay
  ;[0.1073 0.15 0.141 0.5] Initialisation
  ;;[0.15 0.15 0.15 0.5] Create Dynamic Material and apply to mesh
  (bind _returnvalue (Rendering|Material|CreateDynamicMaterialInstance (Variables|Default|GetCharacterPose) 0 "/Game/MyContent/Materials/NPCMaterial_Inst.NPCMaterial_Inst" "None" :!class /Script/Engine.PrimitiveComponent))
  (Variables|Stats|SetNPCMaterial _returnvalue)
  (Rendering|Material|SetMaterial (Variables|Default|GetCharacterPose) 0 (Variables|Stats|GetNPCMaterial))
  ;;[0.15 0.15 0.15 0.5] Create Temperament Widget
  (bind _aswbp_temperament (Utilities|Casting|CastToWBP_Temperament (UserInterface|GetWidget (Variables|Default|GetWidget))))
  (Variables|UI|SetTemperamentWidget _aswbp_temperament)
  (Variables|/Game/MyContent/Widgets/WBP_Temperament.WBP_Temperament_C|SetOwner _aswbp_temperament self)
  ;;[0.15 0.15 0.15 0.5] Create Timer for Comfort Zone detection
  (bind _returnvalue_2 (Utilities|Time|SetTimerbyEvent (delegate Custom|InterrogateComfortZone) 0.5 true))
  (Variables|ComfortZone|SetComfortZoneTimerRef _returnvalue_2))

(fn ConstructionScript)

(fn GetGroundLocation
  (bind _returnvalue (Transformation|GetActorLocation))
  (bind (_outhit _returnvalue_2) (Collision|LineTraceByChannel _returnvalue (- _returnvalue "0.000000,0.000000,500.000000") "TraceTypeQuery1" false (Utilities|Array|MakeArray self) "None"))
  (if _returnvalue_2
    (return (.ImpactPoint (Collision|BreakHitResult _outhit)))))

(fn IncreaseTemperament
  (bind _output_get (Variables|Stats|SetTemperament (Math|Float|Clamp(Float) (+ (Variables|Stats|GetTemperament) 0.01))))
  (if (>= _output_get 0.9)
    (bind _asnpc_aic (Utilities|Casting|CastToNPC_AIC (AI|GetAIController self)))
    (Gameplay|StateTree|SendStateTreeEvent (Variables|/Game/MyContent/AI/Controllers/NPC_AIC.NPC_AIC_C|GetStateTreeAI _asnpc_aic) (Utilities|Struct|MakeStateTreeEvent "(TagName=\"Actions.Retreat\")") :!class /Script/GameplayStateTreeModule.StateTreeComponent)))

(fn DecreaseTemperament
  (Variables|Stats|SetTemperament (Math|Float|Clamp(Float) (- (Variables|Stats|GetTemperament) 0.01))))

(fn CharacterRef
  (return self))